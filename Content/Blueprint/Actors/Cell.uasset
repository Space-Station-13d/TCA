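; Board cell actor for a two-player, unit-based game, with a black or white material set at construction.
; Left clicks are forwarded to the custom game mode, and attaching a unit links it and the cell both ways.
; Occupancy and owner queries treat units marked for death as absent.
; Per-player defender aura flags are rebuilt from affecting defenders, counting only those marked for death as written.
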(event `OnUnitAttachedToCell`
  (params (Unit :type "/Game/Blueprint/Actors/Unit/Unit Object Reference"))
  ;[1 1 1] Unit enters cell
  (bind _output_get (set `self.Unit` Unit))
  (set `/Game/Blueprint/Actors/Unit/Unit.Cell` self _output_get))

(event `self.ReceiveActorOnClicked`
  (params (ButtonPressed :type "Key Structure" :default "AnyKey"))
  ;[1 1 1] Click handler
  (if (== ButtonPressed "LeftMouseButton")
    (`/Game/Blueprint/Systems/CustomGameMode.OnCellClicked` (`/Game/Blueprint/UtilityFunctions.Get Custom Game Mode`) self)))

(fn `ContainsUnit`
  (returns (ContainsUnit :type Boolean))
  (bind _unit (`self.Unit`))
  (if (`KismetSystemLibrary.IsValid` _unit)
    (return (not (`/Game/Blueprint/Actors/Unit/Unit.MarkedForDeath` _unit)))
    (else
      (return false))))

(fn `GetUnitPlayerIfAny`
  (returns (ContainsUnit :type Boolean) (Player :type "/Game/Blueprint/Enums/Player Enum"))
  (if (`self.ContainsUnit`)
    (return true (`/Game/Blueprint/Actors/Unit/Unit.Owning Player` (`self.Unit`)))
    (else
      (return false "NewEnumerator0"))))

(fn `RecalculateDefenderAura`
  (set `self.Defender Aura Player 2` false)
  (set `self.Defender Aura Player 1` false)
  (for _array_element (`self.AffectingDefenders`)
    (`/Engine/EditorBlueprintResources/StandardMacros.IsValid` _array_element
      (:`Is Valid`
        (if (`/Game/Blueprint/Actors/Unit/Unit.MarkedForDeath` _array_element)
          (switch `/Game/Blueprint/Enums/Player` (`/Game/Blueprint/Actors/Unit/Unit.Owning Player` _array_element)
            (:`NewEnumerator0`
              (set `self.Defender Aura Player 1` true))
            (:`NewEnumerator1`
              (set `self.Defender Aura Player 2` true)))))))
  (return))

(fn `UserConstructionScript`
  (bind _cube (`self.Cube`))
  (if (`self.Is Black`)
    (`PrimitiveComponent.SetMaterial` _cube 0 "/Game/Materials/BlackCell.BlackCell")
    (else
      (`PrimitiveComponent.SetMaterial` _cube 0 "/Game/Materials/WhiteCell.WhiteCell"))))