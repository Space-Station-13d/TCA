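; Game mode for a grid-based tactics game, handling unit selection, movement and attacks.
; Left-clicking a unit caches and highlights movable cells and adjacent attackable enemies from the scene's Grid; cell clicks move it, right-clicks attack.
; Unit type and status effects alter ranges, highlights and targets, with one type hitting all targets via a copied array to survive actor destruction.
; Moves, deaths and explicit requests refresh the cached options.
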(event `self.ReceiveBeginPlay`
  (bind (_grid _found) (`/Game/Blueprint/UtilityFunctions.TryFindGridInScene`))
  ;[1 1 1] Setup
  (if _found
    (set `self.Grid` _grid)
    (else
      (`KismetSystemLibrary.PrintText` "Could not set up grid in game mode!"))))

(event `OnUnitClickedLMB`
  (params (Unit :type "/Game/Blueprint/Actors/Unit/Unit Object Reference"))
  ;[1 1 1] Unit selection
  (`self.Clear Currently Selected Unit`)
  (set `self.Currently Selected Unit` Unit)
  (`KismetSystemLibrary.PrintText` (`|FormatText` "{Unit} is now selected." (`/Game/Blueprint/Actors/Unit/Unit.ToText` Unit)))
  (`self.Calculate Movable Cells`)
  (`self.Calculate Attackable Units`))

(event `OnUnitClickedRMB`
  (params (Unit :type "/Game/Blueprint/Actors/Unit/Unit Object Reference"))
  (bind _currently_selected_unit (`self.Currently Selected Unit`))
  ;[1 1 1] Attack
  (if (and (`|EnumInequality` (`/Game/Blueprint/Actors/Unit/Unit.Owning Player` Unit) (`/Game/Blueprint/Actors/Unit/Unit.Owning Player` _currently_selected_unit)) (`KismetArrayLibrary.Array_Contains` (`self.Currently Selected Unit's Attackable Units`) Unit))
    (if (`|EnumEquality` (`/Game/Blueprint/Actors/Unit/Unit.Type` _currently_selected_unit) "NewEnumerator3")
      (bind _output_get (set `self.Local_TemporaryAttackableArray` (`self.Currently Selected Unit's Attackable Units`))) ; Done to avoid foreach problems when\ndestroying the actors inside list.
      (for _array_element _output_get
        (`/Game/Blueprint/Actors/Unit/Unit.OnAttack` (`self.Currently Selected Unit`) _array_element))
      (else
        (`/Game/Blueprint/Actors/Unit/Unit.OnAttack` _currently_selected_unit Unit)))))

(event `OnCellClicked`
  (params (Cell :type "/Game/Blueprint/Actors/Cell Object Reference"))
  ;[1 1 1] Movement
  (`KismetSystemLibrary.PrintText` (`|FormatText` "Cell at {X} {Y} clicked. Its index is {Index}" (`/Game/Blueprint/Actors/Cell.X` Cell) (`/Game/Blueprint/Actors/Cell.Y` Cell) (`KismetArrayLibrary.Array_Find` (`/Game/Blueprint/Actors/Grid.Cells` (`self.Grid`)) Cell)))
  (if (`KismetArrayLibrary.Array_Contains` (`self.Currently Selected Unit's Movable Cells`) Cell)
    (`self.Clear Movable Cells`)
    (`self.Clear Attackable Units`)
    (`/Game/Blueprint/Actors/Unit/Unit.MoveToCell` (`self.Currently Selected Unit`) Cell)
    (`self.Calculate Movable Cells`)
    (`self.Calculate Attackable Units`)))

(event `OnUnitDeath`
  (params (Unit :type "/Game/Blueprint/Actors/Unit/Unit Object Reference"))
  ;[1 1 1] Unit death
  (bind _returnvalue (`KismetArrayLibrary.Array_RemoveItem` (`self.Currently Selected Unit's Attackable Units`) Unit))
  (if _returnvalue
    (`self.Clear Movable Cells`)
    (`self.Calculate Movable Cells`)))

(event `OnRequestRecalculateEverything`
  ;[1 1 1] THROW IT ALL OUT!
  (`self.Clear Movable Cells`)
  (`self.Clear Attackable Units`)
  (`self.Calculate Movable Cells`)
  (`self.Calculate Attackable Units`))

(fn `Calculate Attackable Units`
  (bind _currently_selected_unit (`self.Currently Selected Unit`))
  (bind _currently_selected_unit_2 (`self.Currently Selected Unit`))
  (`KismetArrayLibrary.Array_Clear` (`self.Currently Selected Unit's Attackable Units`))
  (for _array_element (`/Game/Blueprint/Actors/Grid.GetAccessibleCellsByCenterAndRange` (`self.Grid`) (`/Game/Blueprint/Actors/Unit/Unit.Cell` _currently_selected_unit) 1 false false (`/Game/Blueprint/Actors/Unit/Unit.Owning Player` _currently_selected_unit) false true false)
    (if (`/Game/Blueprint/Actors/Cell.ContainsUnit` _array_element)
      ;[1 1 1] Blind effect calculation
      (if (`|EnumEquality` (`/Game/Blueprint/Actors/Unit/UnitDefenceComponent.CurrentEffect` (`/Game/Blueprint/Actors/Unit/Unit.UnitDefenceComponent` _currently_selected_unit_2)) "NewEnumerator2")
        (if (`/Game/Blueprint/Actors/Grid.IsAllyAdjacentToCell` (`self.Grid`) _array_element _currently_selected_unit_2)
          (bind _unit (`/Game/Blueprint/Actors/Cell.Unit` _array_element))
          (`KismetArrayLibrary.Array_Add` (`self.Currently Selected Unit's Attackable Units`) _unit :!label _label)
          (`SceneComponent.SetVisibility` (`/Game/Blueprint/Actors/Unit/Unit.Overlay` _unit) true false))
        (else
          (goto _label)))))
  (return))

(fn `Calculate Movable Cells`
  (bind _currently_selected_unit (`self.Currently Selected Unit`))
  (bind _currently_selected_unit_2 (`self.Currently Selected Unit`))
  (bind _output_get (set `self.Currently Selected Unit's Movable Cells` (`/Game/Blueprint/Actors/Grid.GetAccessibleCellsByCenterAndRange` (`self.Grid`) (`/Game/Blueprint/Actors/Unit/Unit.Cell` _currently_selected_unit_2) (`/Game/Blueprint/Actors/Unit/Unit.Speed` _currently_selected_unit_2) (`|EnumEquality` (`/Game/Blueprint/Actors/Unit/Unit.Type` _currently_selected_unit_2) "NewEnumerator2") false (`/Game/Blueprint/Actors/Unit/Unit.Owning Player` _currently_selected_unit_2) false false (`|EnumEquality` (`/Game/Blueprint/Actors/Unit/UnitDefenceComponent.CurrentEffect` (`/Game/Blueprint/Actors/Unit/Unit.UnitDefenceComponent` _currently_selected_unit_2)) "NewEnumerator5"))))
  (for _array_element _output_get
    ;[1 1 1] Paranoia effect calculation
    (if (`|EnumEquality` (`/Game/Blueprint/Actors/Unit/UnitDefenceComponent.CurrentEffect` (`/Game/Blueprint/Actors/Unit/Unit.UnitDefenceComponent` _currently_selected_unit)) "NewEnumerator1")
      (if (not (`/Game/Blueprint/Actors/Grid.IsAllyAdjacentToCell` (`self.Grid`) _array_element _currently_selected_unit))
        (`SceneComponent.SetVisibility` (`/Game/Blueprint/Actors/Cell.Overlay` _array_element) true false :!label _label))
      (else
        (goto _label))))
  (return))

(fn `Clear Attackable Units`
  (bind _currently_selected_unit_s_attackable_units (`self.Currently Selected Unit's Attackable Units`))
  (for _array_element _currently_selected_unit_s_attackable_units
    (`SceneComponent.SetVisibility` (`/Game/Blueprint/Actors/Unit/Unit.Overlay` _array_element) false false))
  (`KismetArrayLibrary.Array_Clear` _currently_selected_unit_s_attackable_units))

(fn `Clear Currently Selected Unit`
  (set `self.Currently Selected Unit` null)
  (`self.Clear Movable Cells`)
  (`self.Clear Attackable Units`))

(fn `Clear Movable Cells`
  (bind _currently_selected_unit_s_movable_cells (`self.Currently Selected Unit's Movable Cells`))
  (for _array_element _currently_selected_unit_s_movable_cells
    (`SceneComponent.SetVisibility` (`/Game/Blueprint/Actors/Cell.Overlay` _array_element) false false))
  (`KismetArrayLibrary.Array_Clear` _currently_selected_unit_s_movable_cells))

(fn `UserConstructionScript`)