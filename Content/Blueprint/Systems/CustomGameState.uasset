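; CustomGameState holds match-wide data for a two-player game: the round number, plus each player's classes and player state.
; Helper functions increment the round and get or set data by player, with Player 2's state falling back to Player 1's when invalid.
; PostLogin and StartGame are stubs: one checks the first controller's CustomHud and Army without acting on a valid result, the other prints a debug string.
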(event `Post Login`
  (`/Engine/EditorBlueprintResources/StandardMacros.Can Execute Cosmetic Events` ; AKA do we have HUDs for player 0
    (:`True`
      (bind _ascustom_hud (cast `/Game/Blueprint/HUD/CustomHud` (`PlayerController.GetHUD` (`GameplayStatics.GetPlayerController` 0)))
        (:`then`
          (`/Engine/EditorBlueprintResources/StandardMacros.IsValid` (`/Game/Blueprint/HUD/CustomHud.Army` _ascustom_hud)))
        (:`CastFailed`
          (`KismetSystemLibrary.PrintString` "I somehow have no CustomHUD."))))))

(event `StartGame`
  (`KismetSystemLibrary.PrintString` "Hello"))

(fn `Get Player Classes`
  (params (Index :type "/Game/Blueprint/Enums/Player Enum"))
  (returns (Classes :type "Array of /Game/Blueprint/Enums/UnitClasses Enum"))
  (return (select `/Game/Blueprint/Enums/Player` Index :`NewEnumerator0` (`self.Player 1 Classes`) :`NewEnumerator1` (`self.Player 2 Classes`))))

(fn `Get Player State`
  (params (Selection :type "/Game/Blueprint/Enums/Player Enum"))
  (returns (State :type "/Game/Blueprint/Systems/CustomPlayerState Object Reference"))
  (switch `/Game/Blueprint/Enums/Player` Selection
    (:`NewEnumerator0`
      (return (`self.Player 1 State`)))
    (:`NewEnumerator1`
      (`/Engine/EditorBlueprintResources/StandardMacros.IsValid` (`self.Player 2 State`)
        (:`Is Valid`
          (return (`self.Player 2 State`)))
        (:`Is Not Valid`
          (return (`self.Player 1 State`)))))))

(fn `Increment Round Number`
  (`/Engine/EditorBlueprintResources/StandardMacros.IncrementInt` (`self.Round Number`)))

(fn `Set Player Classes`
  (params (Player :type "/Game/Blueprint/Enums/Player Enum") (Classes :type "Array of /Game/Blueprint/Enums/UnitClasses Enum"))
  (switch `/Game/Blueprint/Enums/Player` Player
    (:`NewEnumerator0`
      (set `self.Player 1 Classes` Classes))
    (:`NewEnumerator1`
      (set `self.Player 2 Classes` Classes))))

(fn `UserConstructionScript`)