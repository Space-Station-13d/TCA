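; Game manager for grid-based tactics that tracks the selected unit and highlights where it can move and whom it can attack.
; Grid range queries use the unit's speed, type, side and status effect for movement, and range 1 for attacks.
; Paranoia hides cell highlights next to allies without removing those cells, while Blind limits targets to those next to allies.
; Clear functions hide overlays and empty cached lists; level load/exit events are empty.
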(event `OnMainLevelLoad`)

(event `OnMainLevelExit`)

(fn `CalculateAttackableUnits`
  (locals (NewLocalVar_0 :type Boolean))
  (bind _currentlyselectedunit (`self.CurrentlySelectedUnit`))
  (bind _currentlyselectedunit_2 (`self.CurrentlySelectedUnit`))
  (`KismetArrayLibrary.Array_Clear` (`self.CurrentlySelectedUnit'sAttackableUnits`))
  (for _array_element (`/Game/Blueprint/Actors/Grid.GetAccessibleCellsByCenterAndRange` (`self.Grid`) (`/Game/Blueprint/Actors/Unit/Unit.Cell` _currentlyselectedunit) 1 false false (`/Game/Blueprint/Actors/Unit/Unit.IsBlack` _currentlyselectedunit) false true false)
    (if (`/Game/Blueprint/Actors/Cell.ContainsUnit` _array_element)
      ;[1 1 1] Blind effect calculation
      (if (`|EnumEquality` (`/Game/Blueprint/Actors/Unit/UnitDefenceComponent.CurrentEffect` (`/Game/Blueprint/Actors/Unit/Unit.UnitDefenceComponent` _currentlyselectedunit_2)) "NewEnumerator2")
        (if (`/Game/Blueprint/Actors/Grid.IsAllyAdjacentToCell` (`self.Grid`) _array_element _currentlyselectedunit_2)
          (bind _unit (`/Game/Blueprint/Actors/Cell.Unit` _array_element))
          (`KismetArrayLibrary.Array_Add` (`self.CurrentlySelectedUnit'sAttackableUnits`) _unit :!label _label)
          (`SceneComponent.SetVisibility` (`/Game/Blueprint/Actors/Unit/Unit.Overlay` _unit) true false))
        (else
          (goto _label)))))
  (return))

(fn `CalculateMovableCells`
  (bind _currentlyselectedunit (`self.CurrentlySelectedUnit`))
  (bind _currentlyselectedunit_2 (`self.CurrentlySelectedUnit`))
  (bind _output_get (set `self.CurrentlySelectedUnit'sMovableCells` (`/Game/Blueprint/Actors/Grid.GetAccessibleCellsByCenterAndRange` (`self.Grid`) (`/Game/Blueprint/Actors/Unit/Unit.Cell` _currentlyselectedunit_2) (`/Game/Blueprint/Actors/Unit/Unit.Speed` _currentlyselectedunit_2) (`|EnumEquality` (`/Game/Blueprint/Actors/Unit/Unit.Type` _currentlyselectedunit_2) "NewEnumerator2") false (`/Game/Blueprint/Actors/Unit/Unit.IsBlack` _currentlyselectedunit_2) false false (`|EnumEquality` (`/Game/Blueprint/Actors/Unit/UnitDefenceComponent.CurrentEffect` (`/Game/Blueprint/Actors/Unit/Unit.UnitDefenceComponent` _currentlyselectedunit_2)) "NewEnumerator5"))))
  (for _array_element _output_get
    ;[1 1 1] Paranoia effect calculation
    (if (`|EnumEquality` (`/Game/Blueprint/Actors/Unit/UnitDefenceComponent.CurrentEffect` (`/Game/Blueprint/Actors/Unit/Unit.UnitDefenceComponent` _currentlyselectedunit)) "NewEnumerator1")
      (if (not (`/Game/Blueprint/Actors/Grid.IsAllyAdjacentToCell` (`self.Grid`) _array_element _currentlyselectedunit))
        (`SceneComponent.SetVisibility` (`/Game/Blueprint/Actors/Cell.Overlay` _array_element) true false :!label _label))
      (else
        (goto _label))))
  (return))

(fn `ClearAttackableUnits`
  (bind _currentlyselectedunit_sattackableunits (`self.CurrentlySelectedUnit'sAttackableUnits`))
  (for _array_element _currentlyselectedunit_sattackableunits
    (`SceneComponent.SetVisibility` (`/Game/Blueprint/Actors/Unit/Unit.Overlay` _array_element) false false))
  (`KismetArrayLibrary.Array_Clear` _currentlyselectedunit_sattackableunits)
  (return))

(fn `ClearCurrentlySelectedUnit`
  (set `self.CurrentlySelectedUnit` null)
  (`self.ClearMovableCells`)
  (`self.ClearAttackableUnits`)
  (return))

(fn `ClearMovableCells`
  (bind _currentlyselectedunit_smovablecells (`self.CurrentlySelectedUnit'sMovableCells`))
  (for _array_element _currentlyselectedunit_smovablecells
    (`SceneComponent.SetVisibility` (`/Game/Blueprint/Actors/Cell.Overlay` _array_element) false false))
  (`KismetArrayLibrary.Array_Clear` _currentlyselectedunit_smovablecells)
  (return))