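; Utility function library for a two-player, grid-based unit game with White and Black sides.
; Provides cast helpers for the custom game framework classes, Grid and tagged-actor lookups, and player and unit class conversions to names and colors.
; Unit stats come from a data table by enum name, with a default fallback on a missing row.
; Active player is whoever has the higher activated-unit count, with ties alternating by round parity.
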(fn `Class to Color`
  (params (Class :type "/Game/Blueprint/Enums/UnitClasses Enum"))
  (returns (Color :type "LinearColor Structure"))
  (switch `/Game/Blueprint/Enums/UnitClasses` Class
    (:`NewEnumerator0`
      (return (struct :`R` 0.27816 :`G` 0.0047 :`B` 0.47 :`A` 1.0)))
    (:`NewEnumerator1`
      (return (struct :`R` 0.038113 :`G` 0.720376 :`B` 0.735 :`A` 1.0)))
    (:`NewEnumerator2`
      (return (struct :`R` 0.425 :`A` 1.0)))
    (:`NewEnumerator3`
      (return (struct :`R` 0.086961 :`G` 0.485 :`A` 1.0)))
    (:`NewEnumerator4`
      (return (struct :`R` 0.091619 :`G` 0.144346 :`B` 0.5 :`A` 1.0)))
    (:`NewEnumerator5`
      (return (struct :`R` 0.28 :`G` 0.230431 :`B` 0.136964 :`A` 1.0)))))

(fn `ClassToText`
  (params (Class :type "/Game/Blueprint/Enums/UnitClasses Enum"))
  (returns (Name :type Text))
  ;[1 1 1] PJB make a UnitClass enum to Text data table please
  (return (select `/Game/Blueprint/Enums/UnitClasses` Class :`NewEnumerator0` "Mages" :`NewEnumerator1` "Devout" :`NewEnumerator2` "Military" :`NewEnumerator3` "Primal" :`NewEnumerator4` "Shadows" :`NewEnumerator5` "Beasts" :!type "Text")))

(fn `Determine Active Player`
  (params (`Round Number` :type Integer) (`Player One Activated Units` :type Integer) (`Player Two Activated Units` :type Integer))
  (returns (Player :type "/Game/Blueprint/Enums/Player Enum"))
  ;[1 1 1] Round number internally is offset by 1, so this returns White as first player on EVEN rounds
  (`/Engine/EditorBlueprintResources/StandardMacros.CompareInt` `Player One Activated Units` `Player Two Activated Units`
    (:`>`
      _)
    (:`==`
      (if (== (mod `Round Number` 2) 0)
        _
        (else
          (return "NewEnumerator1"))))
    (:`<`
      (return "NewEnumerator1")))
  (return "NewEnumerator0"))

(fn `Get Custom Game Mode`
  (returns (`Custom Game Mode` :type "/Game/Blueprint/Systems/CustomGameMode Object Reference"))
  (bind _ascustom_game_mode (cast `/Game/Blueprint/Systems/CustomGameMode` (`GameplayStatics.GetGameMode` null))
    (:`then`
      _)
    (:`CastFailed`
      (`KismetSystemLibrary.PrintString` null "Game mode isn't a CustomGameMode! PANIC!")))
  (return _ascustom_game_mode))

(fn `Get Custom Game State`
  (returns (State :type "/Game/Blueprint/Systems/CustomGameState Object Reference"))
  (bind _ascustom_game_state (cast `/Game/Blueprint/Systems/CustomGameState` (`GameplayStatics.GetGameState` null))
    (:`then`
      _)
    (:`CastFailed`
      (`KismetSystemLibrary.PrintString` null "Game mode isn't a CustomGameMode! PANIC!")))
  (return _ascustom_game_state))

(fn `Get Custom Player State`
  (params (Controller :type "PlayerController Object Reference"))
  (returns (`AsCustom Player State` :type "/Game/Blueprint/Systems/CustomPlayerState Object Reference"))
  (bind _ascustom_player_state (cast `/Game/Blueprint/Systems/CustomPlayerState` (`Controller.PlayerState` Controller)))
  (return _ascustom_player_state))

(fn `Get First Actor With Tag`
  (params (Tag :type Name))
  (returns (Actor :type "Actor Object Reference"))
  (bind _outactors (`GameplayStatics.GetAllActorsWithTag` null Tag))
  (if (`KismetMathLibrary.Conv_IntToBool` (`KismetArrayLibrary.Array_Length` _outactors))
    (return (`KismetArrayLibrary.Array_Get` _outactors))
    (else
      (return null))))

(fn `Get Random Unit Class`
  (returns (Class :type "/Game/Blueprint/Enums/UnitClasses Enum"))
  (return (cast `/Game/Blueprint/Enums/UnitClasses` (`KismetMathLibrary.Conv_IntToByte` (`KismetMathLibrary.RandomInteger` (enumcount `/Game/Blueprint/Enums/UnitClasses`))))))

(fn `Get Unit Stats For Type`
  (params (Type :type "/Game/Blueprint/Enums/UnitTypes Enum"))
  (returns (Stats :type "/Game/Blueprint/Data/UnitStats Structure"))
  (locals (`Data Row` :type "/Game/Blueprint/Data/UnitStats Structure" :default (struct :`Type` "NewEnumerator0")))
  (bind _returnvalue (`|GetDataTableRow` "/Game/Blueprint/Data/UnitStatsData.UnitStatsData" (`KismetStringLibrary.Conv_StringToName` (`|GetEnumeratorNameAsString` Type)))
    (:`then`
      (set `local.Data Row` _returnvalue))
    (:`RowNotFound`
      (set `local.Data Row` (make `/Game/Blueprint/Data/UnitStats` Type 1 1 1))
      (`KismetSystemLibrary.PrintText` null (`|FormatText` "ERROR! {Type} Does not exist in UnitStatsData!" (`KismetTextLibrary.Conv_StringToText` (`|GetEnumeratorNameAsString` Type))))))
  (return (`local.Data Row`)))

(fn `GetGameManager`
  (returns (`Game Manager` :type "/Game/Blueprint/Systems/GameManager Object Reference"))
  (bind _asgame_manager (cast `/Game/Blueprint/Systems/GameManager` (`GameplayStatics.GetGameInstance` null))
    (:`then`
      (return _asgame_manager))
    (:`CastFailed`
      (`KismetSystemLibrary.PrintText` null "Game instance is not of game manager class. Check project settings.")
      (return null))))

(fn `IntToTextZeroToEmpty`
  (params (Int :type Integer))
  (returns (Text :type Text))
  (switch `int` Int
    (:`Default`
      (return (`KismetTextLibrary.Conv_IntToText` Int)))
    (:`0`
      (return ""))))

(fn `Player To Color`
  (params (Player :type "/Game/Blueprint/Enums/Player Enum"))
  (returns (Color :type "LinearColor Structure"))
  (switch `/Game/Blueprint/Enums/Player` Player
    (:`NewEnumerator0`
      (return (struct :`R` 1.0 :`G` 1.0 :`B` 1.0 :`A` 1.0)))
    (:`NewEnumerator1`
      (return (struct :`A` 1.0)))))

(fn `Player To Name`
  (params (Player :type "/Game/Blueprint/Enums/Player Enum"))
  (returns (Name :type Text))
  (switch `/Game/Blueprint/Enums/Player` Player
    (:`NewEnumerator0`
      (return "White"))
    (:`NewEnumerator1`
      (return "Black"))))

(fn `TryFindGridInScene`
  (returns (Grid :type "/Game/Blueprint/Actors/Grid Object Reference") (Found :type Boolean))
  (bind _outactors (`GameplayStatics.GetAllActorsOfClass` null "/Game/Blueprint/Actors/Grid.Grid_C"))
  (switch `int` (`KismetArrayLibrary.Array_Length` _outactors)
    (:`Default`
      (`KismetSystemLibrary.PrintText` null "Multiple grids found in scene!"))
    (:`0`
      (`KismetSystemLibrary.PrintText` null "No grids found in scene!")
      (return null false))
    (:`1`
      _))
  (return (`KismetArrayLibrary.Array_Get` _outactors) true))